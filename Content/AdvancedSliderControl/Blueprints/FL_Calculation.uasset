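; Blueprint function library of 2D math helpers in the AdvancedSliderControl folder.
; It tests whether a point lies inside an inclusive min/max rectangle and places a point on a circle from a center, radius and angle in degrees, with Z set to zero.
; It also returns the angle in degrees of the direction from point B to point A, using Atan2 on the normalized difference.
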(fn `GetAngleBetweenTwoPoints`
  (params (A :type "Vector2D Structure") (B :type "Vector2D Structure"))
  (returns (`角度` :type "Float (double-precision)"))
  (bind (_returnvalue_x _returnvalue_y) (`KismetMathLibrary.BreakVector2D` (`KismetMathLibrary.Normal2D` (- A B))))
  (return (`KismetMathLibrary.RadiansToDegrees` (`KismetMathLibrary.Atan2` _returnvalue_y _returnvalue_x))))

(fn `GetLocationFromRadiusAndAngle`
  (params (Radius :type "Float (double-precision)") (Angle :type "Float (double-precision)") (SourceLocation :type "Vector Structure"))
  (returns (ReturnValue :type "Vector Structure"))
  (bind _returnvalue (`KismetMathLibrary.DegreesToRadians` (`local.Angle`)))
  (return (`KismetMathLibrary.MakeVector` (+ (.x (`local.SourceLocation`)) (* (`local.Radius`) (`KismetMathLibrary.Cos` _returnvalue))) (+ (.y (`local.SourceLocation`)) (* (`local.Radius`) (`KismetMathLibrary.Sin` _returnvalue))))))

(fn `IsPointInside `
  (params (Min :type "Vector2D Structure") (Max :type "Vector2D Structure") (Position :type "Vector2D Structure"))
  (returns (ReturnValue :type Boolean))
  (bind (_x _y) (`KismetMathLibrary.BreakVector2D` Min))
  (bind (_x_2 _y_2) (`KismetMathLibrary.BreakVector2D` Max))
  (bind (_x_3 _y_3) (`KismetMathLibrary.BreakVector2D` (`local.Position`)))
  (return (and (<= _x_3 _x_2) (<= _y_3 _y_2) (>= _x_3 _x) (>= _y_3 _y))))